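; Showcase game mode that manages switching between UI and game input and provides access to a shared loot manager.
; A counter of open windows sets UI-only input focused on the newest widget, then restores game-only input when the last one closes.
; RefocusUI returns user focus to the last recorded widget while in UI mode.
; The loot manager actor is spawned lazily when its getter finds no valid instance.
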(fn ConstructionScript)

(fn RefocusUI
  (if (Variables|Default|GetisUIMode)
    (Class|Widget|SetUserFocus (Variables|Default|GetLastFocusedWidget) (Game|GetPlayerController 0))))

(fn OnWindowOpened
  (params (newestFocusedWidget :type Widget%20Object%20Reference))
  (Math|Integer|IncrementInt (Variables|Default|GetwindowsOpen)
    (:%20%20
      (Variables|Default|SetisUIMode true)
      (bind _output_get (Variables|Default|SetLastFocusedWidget newestFocusedWidget))
      (Input|SetInputModeUIOnly (Game|GetPlayerController 0) _output_get "LockAlways"))))

(fn OnWindowClosed
  (bind _result (Math|Integer|DecrementInt (Variables|Default|GetwindowsOpen))
    (:%20%20
      (if (<= _result 0)
        (Variables|Default|SetisUIMode false)
        (Input|SetInputModeGameOnly (Game|GetPlayerController 0))))))

(fn CreateLootManager
  (bind _returnvalue (Game|SpawnActorfromClass "/Game/Blueprints/LootSystem/Loot_Manager_BP.Loot_Manager_BP_C" (Math|Transform|MakeTransform "0, 0, 0" "0, 0, 0" "1,1,1") "AlwaysSpawn" 0 0))
  (Variables|Default|SetLoot%20Manager _returnvalue))

(fn GetLootManager
  (Variables|Default|GetLoot%20Manager
    (:then
      _)
    (:else
      (CallFunction|CreateLootManager)))
  (return (Variables|Default|GetLoot%20Manager)))