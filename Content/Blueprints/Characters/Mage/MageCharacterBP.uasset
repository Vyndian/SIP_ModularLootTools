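; Mage player character Blueprint that handles interaction, inventory toggling, quitting and gear equipping.
; Interact messages the first overlapping actor implementing Interact_Interface, and a SceneCapture2D renders only this character.
; Equip checks equippability and level, returns old gear to InventoryComponentACP, then spawns and attaches new gear to its slot's mesh socket and notifies CharScreenACP.
; Slot-indexed switches map gear and sockets, though SetCurrentEquipment omits the neck slot.
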(event EventBeginPlay
  ;[1 1 1] Add the player actor as a "ShowOnyActors" actor element for the scene capture 2D
  (Utilities|Array|Add (Variables|/Script/Engine.SceneCaptureComponent|GetShowOnlyActors (Variables|Default|GetSceneCaptureComponent2D)) self))

(event Collision|EventActorBeginOverlap
  (params (OtherActor :type Actor%20Object%20Reference)))

(event EventTick
  (params (DeltaSeconds :type Float%20%28single-precision%29)))

(event Input|ActionEvents|InputActionInteractAction
  (params (Key :type Key%20Structure :default "None"))
  ;[1 1 1] Handle Inputs
  (:Pressed
    (CallFunction|DoInteract)))

(event Input|ActionEvents|InputActionInventory
  (params (Key :type Key%20Structure :default "None"))
  ;[1 1 1] Handle Inputs
  (:Pressed
    (Default|ToggleInventory (Variables|Default|GetInventoryComponent_aCP))))

(event Input|KeyboardEvents|Escape
  (params (Key :type Key%20Structure :default "None"))
  ;[1 1 1] Handle Inputs
  (:Released
    (Game|QuitGame 0 "Quit" true)))

(fn ConstructionScript
  (|CallParentFunction))

(fn DoInteract
  (bind _array_element (Utilities|Array|ForEachLoopwithBreak (Collision|GetOverlappingActors "/Script/Engine.Actor" :!class /Script/Engine.Actor) :!label _label)
    (:LoopBody
      (if (Utilities|DoesObjectImplementInterface _array_element "/Game/Blueprints/InventorySystem/Interact_Interface.Interact_Interface_C")
        (Class|InteractInterface|Interact(Message) _array_element)
        (goto _label Break)))))

(fn Equip
  (params (itemToEquip :type Item%20Struct%20Structure))
  ;[1 1 1] If the player can equip this item,
  (bind _canequip (CallFunction|CanEquip itemToEquip))
  (if _canequip
    ;[1 1 1] Find the equipment the input item would replace. If there is currently an item in that slot,
    (bind _slot (CallFunction|FindSlotOfItem itemToEquip))
    (bind _output_get (LocalVariables|SetSlot%20of%20Item%20To%20Equip _slot))
    (bind _equipmentinfoundslot (CallFunction|FindEquipmentbySlot _output_get))
    (Utilities|IsValid _equipmentinfoundslot
      (:Is%20Valid
        ;[1 1 1] then unequip that equipment. If unequip successful,
        (bind _success (CallFunction|UnequipbyReference _equipmentinfoundslot))
        (if _success
          _
          (else
            ;[1 1 1] Else, could not unequip current equipment, so unable to equip new equipment.
            (return false))))
      (:Is%20Not%20Valid
        _))
    ;[1 1 1] Get name of socket to equip this to.
    (bind _socketname (CallFunction|FindSocketNamebySlot (LocalVariables|GetSlot%20of%20Item%20To%20Equip)))
    (LocalVariables|SetSocketName _socketname)
    ;[1 1 1] Spawn the equipment at the correct socket, attach to that socket, and set the equipment variable appropriately.
    (bind _returnvalue (Game|SpawnActorfromClass (.equipItemClass (Utilities|Struct|BreakItem_Struct itemToEquip)) (Transformation|GetSocketTransform (Variables|Character|GetMesh) (LocalVariables|GetSocketName) "RTS_World") "AlwaysSpawn" 0 0))
    (Transformation|AttachComponentToComponent _returnvalue (Variables|Character|GetMesh) (LocalVariables|GetSocketName) "SnapToTarget" "SnapToTarget" "SnapToTarget" true)
    (CallFunction|SetCurrentEquipment _returnvalue)
    ;[1 1 1] Update Char screen (if applicable)
    (Default|OnGearChange (Variables|Default|GetCharScreen_aCP) _returnvalue)
    ;[1 1 1] Equip was successful.
    (return true)
    (else
      ;[1 1 1] CanNOT equip.
      (return false))))

(fn CanEquip
  (params (Item_Struct :type Item%20Struct%20Structure%20%28by%20ref%29))
  (bind (_name _description _thumbnail _pickupitemclass _iskeyitem _isstackable _maxstacksize _isconsumable _isequippable _equipitemclass) (Utilities|Struct|BreakItem_Struct Item_Struct))
  ;[1 1 1] If the item is equippable,
  (if _isequippable
    ;[1 1 1] And if the character is high enough level to equip it,
    (if (>= (Variables|Stats|GetcurrentLevel) (.MinLevel (Utilities|GetClassDefaults _equipitemclass)))
      ;[1 1 1] Player can equip.
      (return true)
      (else
        _)))
  ;[1 1 1] Player canNOT equuip.
  (return false))

(fn UnequipbyReference
  (params (itemToUnequip :type Equip%20Item%20BP%20Object%20Reference))
  ;[1 1 1] Turn the item to unequipt into an inventory slot and attempt to add it to the inventory. If successful,
  (bind _success (Default|AddtoInventory (Variables|Default|GetInventoryComponent_aCP) (Utilities|Struct|MakeSlot_Struct (Variables|/Game/Blueprints/MeshBlueprints/Equippable/EquipItem_BP.EquipItem_BP_C|GetInventoryItemStruct itemToUnequip) 1)))
  (if _success
    ;[1 1 1] Destroy the equipped item.
    (Actor|DestroyActor (LocalVariables|GetItemToUnequip))
    (return true)
    (else
      ;[1 1 1] Else, could not add to inventory.
      (return false))))

(fn FindEquipmentbySlot
  (params (SlotIndex :type Integer%20%28by%20ref%29))
  ;[1 1 1] Based on the provided int (slot),
  (switch int SlotIndex
    (:0
      ;[1 1 1] Return to currently equipped gear that is in that slot.
      (LocalVariables|SetFoundEquipment (Variables|Equipment|GetcurrentTorsoGear)))
    (:1
      (LocalVariables|SetFoundEquipment (Variables|Equipment|GetcurrentHeadGear)))
    (:2
      (LocalVariables|SetFoundEquipment (Variables|Equipment|GetcurrentLeftHandGear)))
    (:3
      (LocalVariables|SetFoundEquipment (Variables|Equipment|GetcurrentRightHandGear)))
    (:4
      (LocalVariables|SetFoundEquipment (Variables|Equipment|GetcurrentNeckGear))))
  (return (LocalVariables|GetFoundEquipment)))

(fn FindSlotOfItem
  (params (Item :type Item%20Struct%20Structure%20%28by%20ref%29))
  (return (.equipSlot (Utilities|GetClassDefaults (.equipItemClass (Utilities|Struct|BreakItem_Struct Item))))))

(fn FindSocketNamebySlot
  (params (slot :type Integer))
  (switch int slot
    (:0
      (LocalVariables|Setname "TorsoSocket"))
    (:1
      (LocalVariables|Setname "HeadSocket"))
    (:2
      (LocalVariables|Setname "LeftHandSocket"))
    (:3
      (LocalVariables|Setname "RightHandSocket"))
    (:4
      (LocalVariables|Setname "NeckSocket")))
  (return (LocalVariables|Getname)))

(fn SetCurrentEquipment
  (params (newEquipment :type Equip%20Item%20BP%20Object%20Reference))
  (switch int (Variables|/Game/Blueprints/MeshBlueprints/Equippable/EquipItem_BP.EquipItem_BP_C|GetequipSlot newEquipment)
    (:0
      (Variables|Equipment|SetcurrentTorsoGear newEquipment))
    (:1
      (Variables|Equipment|SetcurrentHeadGear newEquipment))
    (:2
      (Variables|Equipment|SetcurrentLeftHandGear newEquipment))
    (:3
      (Variables|Equipment|SetcurrentRightHandGear newEquipment))))

(fn UnequipbySlot
  (params (slotToUnequip :type Integer))
  ;[1 1 1] Find equipment in that slot and verify it.
  (bind _equipmentinfoundslot (CallFunction|FindEquipmentbySlot slotToUnequip))
  (if (!= _equipmentinfoundslot 0)
    (bind _success (CallFunction|UnequipbyReference _equipmentinfoundslot))
    (return _success)
    (else
      ;[1 1 1] Else, could not verify equipment.
      (return false))))