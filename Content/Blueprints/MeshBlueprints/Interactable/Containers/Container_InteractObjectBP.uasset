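; Lootable container object that fills its inventory with starting items, random loot or both when play begins.
; On reset it gets the LootManager from ShowcaseGameMode, clears InventoryComponent, then writes defaults by slot index.
; Random rolls come from the LootManager until the count or empty slots run out, with item level and quantity clamped against class defaults.
; It reports its creation and destruction to the LootManager.
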(event Custom|On%20Destroyed%20Event
  (params (DestroyedActor :type Actor%20Object%20Reference))
  (Default|ContainerDestroyed (Variables|ObjectReferences|GetLoot%20Manager) self))

(event EventBeginPlay
  (|CallParentFunction)
  (CallFunction|ResetInventoryComponent)
  (Default|ContainerCreated (Variables|ObjectReferences|GetLoot%20Manager) self)
  (Game|BindEventtoOnDestroyed (delegate Custom|On%20Destroyed%20Event)))

(fn ConstructionScript
  (|CallParentFunction))

(fn SettoDefaultLootItems
  (bind _inventorycomponent (Variables|Default|GetInventoryComponent))
  (bind _currentinventory (Variables|/Game/Blueprints/UI/Components/InventoryComponent_aCP.InventoryComponent_aCP_C|GetcurrentInventory _inventorycomponent))
  (for (_array_element _array_index) (Variables|Levers|GetStarting%20Items)
    (Utilities|Array|SetArrayElem _currentinventory _array_index _array_element)
    (for _array_element_2 _currentinventory
      (if (!= (.Quantity (Utilities|Struct|BreakSlot_Struct _array_element_2)) 0)
        _))))

(fn AddRandomLootItems
  (Utilities|FlowControl|ForLoopwithBreak 1 (Variables|Gears|GetNum%20Random%20Loot%20to%20Generate) :!label _label
    (:LoopBody
      (bind _result (Default|HasEmptyStack (Variables|Default|GetInventoryComponent)))
      (if _result
        (bind (_generated_pickupobject _generated_item_level _quantity) (Default|GenerateRandomLootReference (Variables|ObjectReferences|GetLoot%20Manager) (Variables|RandomLootGenerationLevers|GetMin%20Item%20Level) (Variables|RandomLootGenerationLevers|GetMax%20Item%20Level) (Variables|RandomLootGenerationLevers|GetMin%20Quantity) (Variables|RandomLootGenerationLevers|GetMax%20Quantity)))
        (|EnsureNewItemLevelisvalid _generated_pickupobject _generated_item_level)
        (|EnsureNewQuantityisValid _generated_pickupobject _quantity)
        (Default|AddtoInventory (Variables|Default|GetInventoryComponent) (Utilities|Struct|MakeSlot_Struct (Utilities|Struct|MakeItem_Struct (.name (Utilities|GetClassDefaults _generated_pickupobject)) (.description (Utilities|GetClassDefaults _generated_pickupobject)) (.thumbnail (Utilities|GetClassDefaults _generated_pickupobject)) (.pickupitemclass (Utilities|GetClassDefaults _generated_pickupobject)) (.iskeyitem (Utilities|GetClassDefaults _generated_pickupobject)) (.isstackable (Utilities|GetClassDefaults _generated_pickupobject)) (.maxstacksize (Utilities|GetClassDefaults _generated_pickupobject)) (.isconsumable (Utilities|GetClassDefaults _generated_pickupobject)) (.isequippable (Utilities|GetClassDefaults _generated_pickupobject)) (.equipitemclass (Utilities|GetClassDefaults _generated_pickupobject)) (LocalVariables|GetNew%20Item%20Level)) (LocalVariables|GetNew%20Quantity)))
        (else
          (goto _label Break))))))

(fn ResetInventoryComponent
  ;[1 1 1] Get reference to the Loot Manager.
  (bind _asshowcase_game_mode (Utilities|Casting|CastToShowcaseGameMode (Game|GetGameMode)))
  (bind _loot_manager (Default|GetLootManager _asshowcase_game_mode))
  (Variables|ObjectReferences|SetLoot%20Manager _loot_manager)
  ;[1 1 1] Clear the inventory.
  (Default|ClearInventory (Variables|Default|GetInventoryComponent))
  ;[1 1 1] Add default items if applicable.
  (if (Variables|Levers|GetUse%20Default%20Items)
    (CallFunction|SettoDefaultLootItems))
  ;[1 1 1] Add random loot if applicable
  (if (Variables|Levers|GetAdd%20Random%20Items)
    (CallFunction|AddRandomLootItems)))