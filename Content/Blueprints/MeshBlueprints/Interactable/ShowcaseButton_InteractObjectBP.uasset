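; Interactable showcase button that opens a settings screen when the player interacts with it.
; On interaction it creates a settings widget with a reference back to itself and places it centre-aligned on the Mage player controller's HUD canvas.
; Opening and closing notify the showcase game mode, which is fetched and cached on demand.
; A close function removes the widget and clears its reference.
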(event Custom|Interact%20Event
  (CallFunction|OpenSettingsScreen))

(event EventBeginPlay
  (|CallParentFunction)
  (EventDispatchers|BindEventtoInteractDispatcher (delegate Custom|Interact%20Event)))

(fn ConstructionScript
  (|CallParentFunction))

(fn OpenSettingsScreen
  (bind _returnvalue (UserInterface|CreateWidget "/Game/Blueprints/UI/Widgets/ShowcaseSettingsHUD_Widget.ShowcaseSettingsHUD_Widget_C" 0 self))
  (bind _output_get (Variables|Default|SetSettingsWindow _returnvalue))
  (bind _asmage_player_controller (Utilities|Casting|CastToMage_PlayerController (Game|GetPlayerController 0)))
  (bind _hud_widget (Default|GetHUDWidget _asmage_player_controller))
  (bind _returnvalue_2 (Class|CanvasPanel|AddChildtoCanvas (Variables|/Game/Blueprints/UI/Widgets/PlayerHUD_Widget.PlayerHUD_Widget_C|GetHUD_Canvas _hud_widget) _output_get))
  (Class|CanvasPanelSlot|SetAutoSize _returnvalue_2 true)
  (Class|CanvasPanelSlot|SetAlignment _returnvalue_2 "(X=0.500000,Y=0.500000)")
  (Class|CanvasPanelSlot|SetAnchors _returnvalue_2 (Variables|Default|Getanchors))
  (Class|CanvasPanelSlot|SetPosition _returnvalue_2 (Variables|Default|Getoffset))
  (CallFunction|WindowOpened))

(fn WindowOpened
  (params (In%20Widget%20to%20Focus :type Widget%20Object%20Reference))
  (bind _showcasegamemode (Variables|Default|GetShowcaseGameMode)
    (:then
      _)
    (:else
      (CallFunction|FetchGameMode)))
  (Default|OnWindowOpened _showcasegamemode In%20Widget%20to%20Focus))

(fn WindowClosed
  (bind _showcasegamemode (Variables|Default|GetShowcaseGameMode)
    (:then
      _)
    (:else
      (CallFunction|FetchGameMode)))
  (Default|OnWindowClosed _showcasegamemode))

(fn FetchGameMode
  (bind _asshowcase_game_mode (Utilities|Casting|CastToShowcaseGameMode (Game|GetGameMode)))
  (Variables|Default|SetShowcaseGameMode _asshowcase_game_mode))

(fn CloseSettingsScreen
  (bind _settingswindow (Variables|Default|GetSettingsWindow)
    (:then
      (Widget|RemovefromParent _settingswindow)
      (Variables|Default|SetSettingsWindow 0)
      (CallFunction|WindowClosed))
    (:else)))