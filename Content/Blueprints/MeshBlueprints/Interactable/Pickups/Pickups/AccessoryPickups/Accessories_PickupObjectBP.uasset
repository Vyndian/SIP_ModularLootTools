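; Pickup Blueprint for accessory items that the player equips on use.
; UseItem runs the parent check first and, if it succeeds, casts player 0's character to MageCharacterBP and returns the result of equipping PickupItem.
; If the parent check fails, its result is returned unchanged.
; The event graph holds only disabled stubs, and construction defers to the parent.
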(event EventBeginPlay
  (|CallParentFunction) ; This node is disabled and will not be called.\nDrag off pins to build functionality.
)

(event Collision|EventActorBeginOverlap
  (params (OtherActor :type Actor%20Object%20Reference))
  (|CallParentFunction OtherActor) ; This node is disabled and will not be called.\nDrag off pins to build functionality.
)

(event EventTick
  (params (DeltaSeconds :type Float%20%28single-precision%29))
  (|CallParentFunction DeltaSeconds) ; This node is disabled and will not be called.\nDrag off pins to build functionality.
)

(fn ConstructionScript
  (|CallParentFunction))

(fn UseItem
  (bind _success (|CallParentFunction))
  (if _success
    (bind _asmage_character_bp (Utilities|Casting|CastToMageCharacterBP (Game|GetPlayerCharacter 0)))
    (bind _success_2 (Default|Equip _asmage_character_bp (Variables|Default|GetPickup%20Item)))
    (return _success_2)
    (else
      (return _success))))