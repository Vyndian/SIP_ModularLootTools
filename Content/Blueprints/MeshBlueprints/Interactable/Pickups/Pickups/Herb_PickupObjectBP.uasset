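; Herb pickup Blueprint that heals the player mage when used, built on a parent pickup class.
; UseItem runs the parent logic, then casts the player character to MageCharacterBP and adds HealValue to its health resource component.
; It then spawns a heal particle emitter attached to the player's mesh and returns true.
; The event graph holds only disabled default events.
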(event EventBeginPlay
  (|CallParentFunction) ; This node is disabled and will not be called.\nDrag off pins to build functionality.
)

(event Collision|EventActorBeginOverlap
  (params (OtherActor :type Actor%20Object%20Reference))
  (|CallParentFunction OtherActor) ; This node is disabled and will not be called.\nDrag off pins to build functionality.
)

(event EventTick
  (params (DeltaSeconds :type Float%20%28single-precision%29))
  (|CallParentFunction DeltaSeconds) ; This node is disabled and will not be called.\nDrag off pins to build functionality.
)

(fn ConstructionScript
  (|CallParentFunction))

(fn UseItem
  (|CallParentFunction)
  ;[1 1 1] Get the player and heal them.
  (bind _asmage_character_bp (Utilities|Casting|CastToMageCharacterBP (Game|GetPlayerCharacter 0)))
  (Default|ChangeCurrent (Variables|/Game/Blueprints/Characters/ThirdPersonCharacter.ThirdPersonCharacter_C|GetHealth_ResourceCP _asmage_character_bp) (Variables|Default|GethealValue))
  ;[1 1 1] Spawn the heal particle system at the player's mesh and attach it. It should destroy itself after playing.
  (Effects|SpawnEmitterAttached (Variables|Default|GetHeal_ParticleSystem) (Variables|/Script/Engine.Character|GetMesh _asmage_character_bp) "None")
  (return true))