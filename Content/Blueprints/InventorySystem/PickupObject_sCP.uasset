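; Scene component that lets its owning PickupObject_InteractObjectBP be picked up into the player's inventory.
; On BeginPlay it binds PickupEvent to the owner's interact dispatcher, copies the owner's PickupItem, and unbinds when the owner is destroyed.
; On interaction it adds the item and quantity to player 0's InventoryComponentACP, then destroys the owner if the add succeeds and destroy-on-pickup is enabled.
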(event Custom|OnDestroyed
  (params (DestroyedActor :type Actor%20Object%20Reference))
  ;[1 1 1] Bind the PickupEvent delegate to the InteractDispatcher. Bind OnDestroyed to when this scene component is destroyed to remove the PickupEvent delegate from the InteractDispatcher.
  (EventDispatchers|UnbindEventfromInteractDispatcher (Variables|Default|GetparentPickupObject) (delegate Custom|PickupEvent)))

(event Custom|PickupEvent
  ;[1 1 1] Bind the PickupEvent delegate to the InteractDispatcher. Bind OnDestroyed to when this scene component is destroyed to remove the PickupEvent delegate from the InteractDispatcher.
  (CallFunction|Pickup))

(event EventBeginPlay
  ;[1 1 1] Get Reference to parent actor
  (bind _aspickup_object_interact_object_bp (Utilities|Casting|CastToPickupObject_InteractObjectBP (Components|GetOwner)))
  (bind _output_get (Variables|Default|SetparentPickupObject _aspickup_object_interact_object_bp))
  ;[1 1 1] Bind the PickupEvent delegate to the InteractDispatcher. Bind OnDestroyed to when this scene component is destroyed to remove the PickupEvent delegate from the InteractDispatcher.
  (EventDispatchers|BindEventtoInteractDispatcher _output_get (delegate Custom|PickupEvent))
  (Game|BindEventtoOnDestroyed (Components|GetOwner) (delegate Custom|OnDestroyed))
  ;[1 1 1] Set this component's pickupItem based on the pickupObject default
  (Variables|Default|SetpickupItem (Variables|/Game/Blueprints/MeshBlueprints/Interactable/Pickups/PickupObject_InteractObjectBP.PickupObject_InteractObjectBP_C|GetPickup%20Item (Variables|Default|GetparentPickupObject))))

(fn Pickup
  ;[1 1 1] Get reference to player & inventory
  (bind _asthird_person_character (Utilities|Casting|CastToThirdPersonCharacter (Game|Player|GetPlayerPawn 0)))
  (bind _output_get (LocalVariables|Setplayer _asthird_person_character))
  (bind _output_get_2 (LocalVariables|SetplayerInventory (Variables|/Game/Blueprints/Characters/ThirdPersonCharacter.ThirdPersonCharacter_C|GetInventoryComponent_aCP _output_get)))
  ;[1 1 1] Pick up the item
  (bind _success (Default|AddtoInventory _output_get_2 (Utilities|Struct|MakeSlot_Struct (Variables|Default|GetpickupItem) (Variables|Default|GetQuantityOnPickup))))
  ;[1 1 1] Destroy if pickup succeeded AND this pickupObject set to destroy on pickup
  (|DestroyPickup? _success))